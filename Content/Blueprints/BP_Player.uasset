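; Player pawn Blueprint for a gun-wielding character, mainly linking the equipped weapon to the HUD.
; On BeginPlay it gets the main HUD from SPlayerController_BP and, if EquippedGun is valid, pushes its magazine and total ammo to the display.
; Tick and the IA_Sprint input are empty, and leftover weapon-spawn, ammo debug print and Aim-stop nodes are disconnected and never run.
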(event Input|EnhancedActionEvents|EnhancedInputActionIA_Sprint
  (params (ActionValue :type Boolean) (ElapsedSeconds :type Float%20%28double-precision%29) (TriggeredSeconds :type Float%20%28double-precision%29) (InputAction :type Input%20Action%20Object%20Reference :default "/Game/Input/IA_Sprint.IA_Sprint")))

(event EventTick
  (params (DeltaSeconds :type Float%20%28single-precision%29)))

(event EventBeginPlay
  (bind _equippedgun (Variables|Default|GetEquippedGun))
  (bind _assplayer_controller_bp (Utilities|Casting|CastToSPlayerController_BP (Pawn|GetController self)))
  (bind _output_get (Variables|Default|SetMainUI (Variables|/Game/Blueprints/SPlayerController_BP.SPlayerController_BP_C|GetMainHudRef _assplayer_controller_bp)))
  (Utilities|IsValid _equippedgun
    (:Is%20Valid
      (Class|MainWidget|UpdateAmmo _output_get (Class|SGunBase|GetRestMagAmmo _equippedgun) (Variables|/Script/Stellar_Front.SGunBase|GetTotalAmmo _equippedgun)))))

(fn ConstructionScript)